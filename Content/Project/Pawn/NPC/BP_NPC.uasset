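; BP_NPC is a modular NPC character that loads its name, outfit meshes, location and type from a data table.
; The construction script makes clothing and hair meshes follow the Body pose, and Tick yaws a spring arm toward the player camera.
; NPCMove walks it to a random reachable point near a target.
; A mark widget shows name, typed soliloquy and quest state from the player's Playfab component, which also updates the dialogue button text.
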(event EventBeginPlay
  (|CallParentFunction)
  (Pawn|SpawnDefaultController))

(event EventNPCMove
  (params (FLoc :type Vector :default "0, 0, 0"))
  (bind _returnvalue (Class|NavigationSystemV1|GetNavigationSystem))
  (bind _randomlocation (AI|Navigation|GetRandomReachablePointinRadius _returnvalue FLoc 15.0 0 0))
  ;[1 1 1] 코멘트
  (Variables|Default|SetPlayerAnimState "Walk")
  (bind _movementresult (AI|AIMoveTo self (Math|Vector|MakeVector (.x _randomlocation) (.y _randomlocation) (.z _randomlocation)) 0 15.0 true)
    (:OnSuccess
      (Variables|Default|SetPlayerAnimState "Idle"))
    (:OnFail
      (switch Utilities|FlowControl|Switch|SwitchonEPathFollowingResult _movementresult
        (:Blocked
          _)
        (:OffPath
          _)
        (:Aborted
          _)
        (:Invalid
          _))
      (Development|PrintString (Utilities|String|Append "error :" (Utilities|String|EnumtoString _movementresult))))))

(event EventInitNPC
  (params (ID :type String))
  (bind _returnvalue (Utilities|GetDataTableRow "/Game/Project/DataTable/NPC/Data_NPC.Data_NPC" (Utilities|String|StringToName ID))
    (:then
      (Variables|Default|SetCharacterName (Utilities|Text|ToText(Name) (.NpcName (Utilities|Struct|BreakNpcCustomizing_Struct _returnvalue))))
      (Components|SkinnedMesh|SetSkinnedAssetandUpdate (Variables|Default|GetHair) (.Hair (Utilities|Struct|BreakNpcCustomizing_Struct _returnvalue)) true)
      (Components|SkinnedMesh|SetSkinnedAssetandUpdate (Variables|Default|GetTop) (.Top (Utilities|Struct|BreakNpcCustomizing_Struct _returnvalue)) true)
      (Components|SkinnedMesh|SetSkinnedAssetandUpdate (Variables|Default|GetBottoms) (.Bottoms (Utilities|Struct|BreakNpcCustomizing_Struct _returnvalue)) true)
      (Components|SkinnedMesh|SetSkinnedAssetandUpdate (Variables|Default|GetShoes) (.Shoes (Utilities|Struct|BreakNpcCustomizing_Struct _returnvalue)) true)
      (Transformation|SetActorLocation (.NpcLocation (Utilities|Struct|BreakNpcCustomizing_Struct _returnvalue)) false false)
      (Variables|Default|SeteNPCType (.Type (Utilities|Struct|BreakNpcCustomizing_Struct _returnvalue))))))

(event EventTick
  (params (DeltaSeconds :type Float%20%28single-precision%29))
  (bind _returnvalue (Game|GetPlayerController 0))
  (bind _springarm (Variables|Default|GetSpringArm))
  (bind _returnvalue_2 (Transformation|GetWorldLocation _springarm))
  (bind _playercameramanager (Variables|/Script/Engine.PlayerController|GetPlayerCameraManager _returnvalue))
  (bind _returnvalue_3 (Camera|GetCameraLocation _playercameramanager))
  (bind _returnvalue_4 (Math|Vector|MakeVector (.x _returnvalue_2) (.y _returnvalue_2) 0.0))
  (bind _returnvalue_5 (Math|Vector|MakeVector (.x _returnvalue_3) (.y _returnvalue_3) 0.0))
  (bind _returnvalue_6 (Math|Rotator|FindLookatRotation _returnvalue_4 _returnvalue_5))
  (Utilities|IsValid _returnvalue
    (:Is%20Valid
      (Transformation|SetWorldRotation (Variables|Default|GetSpringArm) (Math|Rotator|MakeRotator (.roll _returnvalue_6) (.pitch _returnvalue_6) (.yaw _returnvalue_6)) false false))))

(fn ConstructionScript
  (Components|SkinnedMesh|SetLeaderPoseComponent (Variables|Default|GetTop) (Variables|Default|GetBody) false false))

(fn SetNpcName
  (params (NpcName :type Text))
  ;[1 1 1] Npc 이름 설정
  (bind _aswb_npc_mark (Utilities|Casting|CastToWB_NpcMark (UserInterface|GetWidget (Variables|Default|GetWidget_NpcMark))))
  (Default|SetNpcName _aswb_npc_mark NpcName))

(fn QuestableNpc
  (params (QuestName :type String))
  ;[1 1 1] 퀘스트 가능한 Npc 인가 표시
  (bind _asbp_login_pawn (Utilities|Casting|CastToBP_LoginPawn (Game|Player|GetPlayerPawn 0)))
  (bind _returnvalue (Class|ActorComponentPlayfab|QuestCheckCondition (Variables|/Game/Project/Pawn/Solaseado/BP_LoginPawn.BP_LoginPawn_C|GetActorComponent_Playfab _asbp_login_pawn) QuestName))
  (switch Utilities|FlowControl|Switch|Switchonenum_Quest_Condition _returnvalue
    (:NotStart
      (bind _aswb_npc_mark (Utilities|Casting|CastToWB_NpcMark (UserInterface|GetWidget (Variables|Default|GetWidget_NpcMark))))
      (Default|ExclamationMarkVisibility _aswb_npc_mark "Visible" "(R=1.000000,G=1.000000,B=1.000000,A=1.000000)")
      (bind _asgm_solaseado (Utilities|Casting|CastToGM_Solaseado (Game|GetGameMode)))
      (Rendering|Components|TextRender|SetText (Variables|/Game/Project/Widget/Menu/WB_MainMenu.WB_MainMenu_C|GetTextBlock_DialogueButton (Variables|/Game/Project/World/GM_Solaseado.GM_Solaseado_C|GetWB_MainMenu _asgm_solaseado)) "대화하기(퀘스트 가능)"))
    (:IsDoing
      (bind _aswb_npc_mark_2 (Utilities|Casting|CastToWB_NpcMark (UserInterface|GetWidget (Variables|Default|GetWidget_NpcMark)) :!label _label))
      (Default|ExclamationMarkVisibility _aswb_npc_mark_2 "Visible" "(R=0.000000,G=1.000000,B=0.500000,A=1.000000)")
      (bind _asgm_solaseado_2 (Utilities|Casting|CastToGM_Solaseado (Game|GetGameMode)))
      (Rendering|Components|TextRender|SetText (Variables|/Game/Project/Widget/Menu/WB_MainMenu.WB_MainMenu_C|GetTextBlock_DialogueButton (Variables|/Game/Project/World/GM_Solaseado.GM_Solaseado_C|GetWB_MainMenu _asgm_solaseado_2)) "대화하기(퀘스트 진행 중)"))
    (:LastFinished
      (goto _label))
    (:IsComplete
      (bind _aswb_npc_mark_3 (Utilities|Casting|CastToWB_NpcMark (UserInterface|GetWidget (Variables|Default|GetWidget_NpcMark))))
      (Class|WidgetNpcMark|ExclamationMarkVisibility _aswb_npc_mark_3 "Collapsed")
      (bind _asgm_solaseado_3 (Utilities|Casting|CastToGM_Solaseado (Game|GetGameMode)))
      (Rendering|Components|TextRender|SetText (Variables|/Game/Project/Widget/Menu/WB_MainMenu.WB_MainMenu_C|GetTextBlock_DialogueButton (Variables|/Game/Project/World/GM_Solaseado.GM_Solaseado_C|GetWB_MainMenu _asgm_solaseado_3)) "대화하기(퀘스트 완료)"))))

(fn SetNpcMarkVisibility
  (params (Visibility :type Boolean))
  ;[1 1 1] Npc 마크 설정
  (Rendering|SetVisibility (Variables|Default|GetWidget_NpcMark) Visibility false))

(fn SetSoliloquyText
  (params (SoliloquyText :type Text))
  ;[1 1 1] 혼잣말 텍스트 설정
  (bind _aswb_npc_mark (Utilities|Casting|CastToWB_NpcMark (UserInterface|GetWidget (Variables|Default|GetWidget_NpcMark))))
  ;[1 1 1] 타이핑 효과
  (Default|WriteSoliloquy _aswb_npc_mark (Utilities|String|ToString(Text) SoliloquyText)))

(fn SetVisibleSoliloquyBox
  (params (Visible :type Boolean))
  ;[1 1 1] 혼잣말 박스 설정
  (bind _aswb_npc_mark (Utilities|Casting|CastToWB_NpcMark (UserInterface|GetWidget (Variables|Default|GetWidget_NpcMark))))
  (Default|SetVisibleSoliloquyBox _aswb_npc_mark Visible))