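; Game mode for Solaseado that directs level flow, top-level UI and online service actors.
; On BeginPlay it loads Intro and spawns the HTTP actor; each stream-finish event moves the pawn to its tag-matched PlayerStart, syncs Photon, then opens intro, customization or main menu.
; Events create login, loading, popup and dialogue widgets, set up pawn camera and input, and spawn Photon cloud, chat and voice clients.
; NPC functions route main-menu button presses into dialogue and quests.
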(event Custom|SpawnHTTP
  ;[1 1 1] http 액터 생성
  ;;[1 1 1] 생성되지 않았으면 생성
  (Utilities|IsValid (Variables|Default|GetHTTPRequestActor)
    (:Is%20Not%20Valid
      (bind _returnvalue (Game|SpawnActorfromClass "/Game/Project/Actor/HTTP/BP_HTTPRequest.BP_HTTPRequest_C" (Math|Transform|MakeTransform "0, 0, 0" "0, 0, 0" "1.000000,1.000000,1.000000") "AlwaysSpawn" "OverrideRootScale" 0 0))
      (Variables|Default|SetHTTPRequestActor _returnvalue))))

(event Custom|Pawn_Visible
  (params (IsVisible :type Boolean))
  ;[1 0.7404 0.5342] 캐릭터 visible처리, Camera Setting
  (bind _asbp_login_pawn (Utilities|Casting|CastToBP_LoginPawn (Game|Player|GetPlayerPawn 0)))
  (Rendering|SetVisibility (Variables|/Script/Test_LidarSample.Pawn_Player|GetRoot _asbp_login_pawn) IsVisible true)
  (Default|DefaultCameraSetting _asbp_login_pawn)
  (bind _aspc_solaseado (Utilities|Casting|CastToPC_Solaseado (Game|GetPlayerController 0)))
  (bind _output_get (Variables|/Game/Project/World/PC_Solaseado.PC_Solaseado_C|SetAs%20BP%20Login%20Pawn _aspc_solaseado _asbp_login_pawn))
  ;[1 1 1] 캐릭터 움직일 수 있게 만드는 시점
  (CallFunction|CameraSetting _output_get)
  (Audio|PlaySound2D "/Game/Project/Sound/M1_BGM_01.M1_BGM_01" 1.0 1.0 0.0 0 0))

(event Custom|OnEndLoading
  (CallFunction|SolaseadoLogin))

(event Custom|UIMainMenu
  (bind _returnvalue (Game|GetPlayerController 0))
  ;[1 1 1] MainMenuWidget 생성
  (Development|PrintString "// Widget :: UIMainMenu")
  (CallFunction|WidgetAllRemove)
  (bind _returnvalue_2 (UserInterface|CreateWidget "/Game/Project/Widget/Menu/WB_MainMenu.WB_MainMenu_C"))
  (bind _output_get (Variables|Default|SetWB_MainMenu _returnvalue_2))
  (UserInterface|Viewport|AddtoViewport _output_get 0)
  (Default|CallEventDispatcherCreateMainMenu)
  (Utilities|FlowControl|Sequence
    (:then_0
      (Utilities|FlowControl|DoOnce false
        (:Completed
          ;[1 0 0] Visible, Camera, BGM Setting
          (CallFunction|PawnVisible true))))
    (:then_1
      (bind _aspc_solaseado (Utilities|Casting|CastToPC_Solaseado _returnvalue))
      (Input|EnableInput _aspc_solaseado _returnvalue)
      ;[1 1 1] Dialogue System Create
      (CallFunction|UIDialogue)
      (Widget|SetVisibility (Variables|Default|GetWB_DialogueSystem) "Collapsed"))))

(event Custom|WidgetCreate_Intro
  ;[1 1 1] Intro Widget 추가
  (Development|PrintString "// Widget :: Intro")
  (CallFunction|WidgetAllRemove)
  (bind _returnvalue (UserInterface|CreateWidget "/Game/Project/Widget/intro/WB_Intro.WB_Intro_C"))
  (bind _output_get (Variables|Default|SetWidget_Intro _returnvalue))
  (UserInterface|Viewport|AddtoViewport _output_get 0))

(event Custom|UIDialogue
  ;[1 1 1] 대화시스템 Widget 생성
  (bind _returnvalue (UserInterface|CreateWidget "/Game/Project/Widget/Popup/WB_DialogueSystem.WB_DialogueSystem_C"))
  (bind _output_get (Variables|Default|SetWB_DialogueSystem _returnvalue))
  (UserInterface|Viewport|AddtoViewport _output_get 0))

(event Custom|Camera_Setting
  (params (LoginPawn :type BP%20Login%20Pawn%20Object%20Reference))
  (bind _returnvalue (Game|GetPlayerController 0))
  ;[1 1 1] 임시 터치인터페이스 활성화
  (Class|PlayerController|ActivateTouchInterface _returnvalue "/Engine/MobileResources/HUD/LeftVirtualJoystickOnly.LeftVirtualJoystickOnly")
  (Pawn|SetControlRotation _returnvalue (Transformation|GetActorRotation LoginPawn))
  (Variables|/Script/Engine.Pawn|SetbUseControllerRotationYaw LoginPawn false)
  (Variables|/Script/Engine.SpringArmComponent|SetbUsePawnControlRotation (Variables|/Game/Project/Pawn/Solaseado/BP_LoginPawn.BP_LoginPawn_C|GetSpringArm LoginPawn) true))

(event Custom|StreamLevelFinish_Event_0
  (params (level :type String))
  ;[0 0.6099 1] // Intro  시작 & 레벨 이동 델리게이트 이벤트 바인딩 / StreamLevelFinish
  ;;[1 1 1] 레벨 이동에 따른 설정 추가 하기
  (CallFunction|SetLevelLoadFinishedEvent level))

(event Custom|Solaseado_Login
  ;[1 1 1] // Login Widget / Intro 이후 로그인 적용
  (bind _returnvalue (UserInterface|CreateWidget "/Game/Project/Widget/WB_SolaseadoLogin.WB_SolaseadoLogin_C"))
  (bind _output_get (Variables|Default|SetWidget_SolaseadoLogin _returnvalue))
  (UserInterface|Viewport|AddtoViewport _output_get 0))

(event Custom|SpawnActor_Photon_All
  (bind _returnvalue (Math|Transform|MakeTransform "0, 0, 0"))
  ;[1 1 1] Photon Spawn All
  (bind _asbp_login_pawn (Utilities|Casting|CastToBP_LoginPawn (Game|Player|GetPlayerPawn 0)))
  (bind _returnvalue_2 (Game|SpawnActorfromClass "/Game/Project/Actor/PhotonClient/BP_SolaseadoPhoton.BP_SolaseadoPhoton_C" _returnvalue "AlwaysSpawn" "OverrideRootScale" 0 0))
  (bind _output_get (Variables|Default|SetPhotonCloud _returnvalue_2))
  (bind _returnvalue_3 (Game|SpawnActorfromClass "/Game/Project/Actor/PhotonChat/PhotonChatClient.PhotonChatClient_C" _returnvalue "AlwaysSpawn" "OverrideRootScale" 0 0))
  (bind _output_get_2 (Variables|Default|SetPhotonChat _returnvalue_3))
  (bind _returnvalue_4 (Game|SpawnActorfromClass "/Game/Project/Actor/PhotonVoice/PhotonVoiceClient.PhotonVoiceClient_C" _returnvalue "AlwaysSpawn" "OverrideRootScale" 0 0))
  (bind _output_get_3 (Variables|Default|SetPhotonVoice _returnvalue_4))
  (Class|ActorPhotonVoice|Connect _output_get_3 (Default|GetUserCharacterName _asbp_login_pawn))
  (Class|ActorPhotonChat|ConnectChat _output_get_2 (Default|GetUserCharacterName _asbp_login_pawn))
  ;;[1 0.2396 0.2396] ConnectComplete=> Cloud룸설정=>
  ;; JoinOrCreateComplete => chat,voice 룸설정
  (Class|ActorSolaseadoPhoton|ConnectLogin _output_get (Default|GetUserCharacterName _asbp_login_pawn)))

(event Custom|WidgetCreate_Loading
  ;[1 1 1] Loading Widget 추가 / SJW
  (Development|PrintString "// Widget :: Loading")
  (CallFunction|WidgetAllRemove)
  (bind _returnvalue (UserInterface|CreateWidget "/Game/Project/Widget/intro/WB_Loading.WB_Loading_C"))
  (bind _output_get (Variables|Default|SetWB_Loading _returnvalue))
  (UserInterface|Viewport|AddtoViewport _output_get 0)
  (EventDispatchers|BindEventtoOnEndLoading _output_get (delegate Custom|OnEndLoading)))

(event Custom|UICustomizing
  ;[1 1 1] CustomizingUI
  (Class|PlayerStateSolaseado|UICustomizing (Class|GameModeBaseSolaseado|GetPlayerStateSolaseado)))

(event Custom|Create_Nickname
  ;[1 1 1] NicknameWidget 생성
  (Utilities|IsValid (Variables|Default|GetWB_Create_Nickname)
    (:Is%20Valid
      (UserInterface|Viewport|AddtoViewport (Variables|Default|GetWB_Create_Nickname) 0))
    (:Is%20Not%20Valid
      (bind _returnvalue (UserInterface|CreateWidget "/Game/Project/Widget/Customizing/WB_CreateNickname.WB_CreateNickname_C"))
      (bind _output_get (Variables|Default|SetWB_Create_Nickname _returnvalue))
      (UserInterface|Viewport|AddtoViewport _output_get 0))))

(event EventWidgetCreatePopup
  ;[1 1 1] Popup위젯 생성
  (Utilities|IsValid (Variables|Default|GetWB_Popup)
    (:Is%20Valid
      (UserInterface|Viewport|AddtoViewport (Variables|Default|GetWB_Popup) 0))
    (:Is%20Not%20Valid
      (bind _returnvalue (UserInterface|CreateWidget "/Game/Project/Widget/Popup/WB_Popup.WB_Popup_C"))
      (bind _output_get (Variables|Default|SetWB_Popup _returnvalue))
      (UserInterface|Viewport|AddtoViewport _output_get 0))))

(event EventBeginPlay
  ;[0 0.6099 1] // Intro  시작 & 레벨 이동 델리게이트 이벤트 바인딩 / StreamLevelFinish
  (EventDispatchers|AssignStreamLevelFinish (delegate Custom|StreamLevelFinish_Event_0))
  ;;[1 1 1] Defualt Level Load // Intro
  (Class|GameModeBaseSolaseado|FastMoveLevel "Intro")
  ;;[1 1 1] HTTP 액터 생성
  (CallFunction|SpawnHTTP))

(event EventInsufficientFundsPopup
  ;[1 1 1] 돈 부족 Popup
  (Class|WidgetPopup|AddPopup (Variables|Default|GetWB_Popup) "Popup1Key" "포인트가 부족해 구매할 수 없습니다." "구매 불가" "Exit" "" "" "닫기" false))

(event Custom|SetNpcDialogueButton
  (params (Enabled :type Boolean) (Visibility :type ESlateVisibility%20Enum :default "Visible") (NpcName :type Name))
  (bind _wb_mainmenu (Variables|Default|GetWB_MainMenu))
  (Default|SetNpcDialogueButton _wb_mainmenu Enabled Visibility)
  (EventDispatchers|BindEventtoEventDispatcherDialogueButton _wb_mainmenu (delegate Custom|EventDispatcherDialogueButton)))

(event Custom|EventDispatcherDialogueButton
  (bind _output_get (Variables|Default|SetNpc%20Name (stale Custom|SetNpcDialogueButton NpcName)))
  (Npc|NpcDialog _output_get))

(fn ConstructionScript)

(fn SetStartPointMoveLocation
  (params (Level :type String))
  (bind _photoncloud (Variables|Default|GetPhotonCloud))
  ;[1 1 1] Level > Player Start tag 비교
  (bind _outactors (Actor|GetAllActorsOfClass "/Script/Engine.PlayerStart"))
  (for _array_element _outactors
    (if (Utilities|Name|Equal(Name) (Variables|/Script/Engine.PlayerStart|GetPlayerStartTag _array_element) (Utilities|String|StringToName Level))
      ;[1 0.2552 0.2552] Pawn Transform = StartPoint
      (Transformation|SetActorTransform (Game|Player|GetPlayerPawn 0) (Math|Transform|MakeTransform (.location (Transformation|GetActorTransform _array_element)) (.rotation (Transformation|GetActorTransform _array_element)) "1.000000,1.000000,1.000000"))
      (Development|PrintString (Utilities|String|Append "// Player Pawn Set Location :: " (Utilities|String|ToString(Name) (Variables|/Script/Engine.PlayerStart|GetPlayerStartTag _array_element))))
      ;[1 1 1] 포톤에 플레이어 위치 갱신
      (Utilities|IsValid _photoncloud
        (:Is%20Valid
          (Class|ActorSolaseadoPhoton|MoveandRotation _photoncloud (.location (Transformation|GetActorTransform _array_element)) (Math|Float|Truncate (.Yaw (Math|Rotator|BreakRotator (.rotation (Transformation|GetActorTransform _array_element))))))
          (return))))))

(fn SetLevelLoadFinishedEvent
  (params (Level :type String))
  (CallFunction|SetStartPointMoveLocation Level)
  (Utilities|Casting|CastToGM_Solaseado (Game|GetGameMode))
  (switch string Level
    (:Intro
      (Development|PrintString "// Check move Level :: Intro")
      (CallFunction|WidgetCreateIntro))
    (:Login
      ;[1 0.1976 0.2175] Login Level 을 임시 커스터마이징 씬으로 활용.
      (CallFunction|UICustomizing))
    (:SimPoly1
      (Development|PrintString "// Check move Level :: inGame ")
      (CallFunction|UIMainMenu))))

(fn WidgetAllRemove
  (params (ExeptionWidget :type User%20Widget%20Object%20Reference))
  (bind _foundwidgets (Widget|GetAllWidgetsOfClass "/Script/UMG.UserWidget" true))
  (for _array_element _foundwidgets
    (if (!= _array_element ExeptionWidget)
      ;[1 1 1] 예외 위젯이 아니라면 모두 지우기
      (Widget|RemovefromParent _array_element))))

(fn NpcDialog
  (params (NpcName :type Name))
  (bind _wb_dialoguesystem (Variables|Default|GetWB_DialogueSystem))
  (Utilities|IsValid _wb_dialoguesystem
    (:Is%20Valid
      (Widget|SetVisibility _wb_dialoguesystem "Visible")
      (Default|StartDialogue _wb_dialoguesystem NpcName)
      (Default|SetUIOnly (Variables|Default|GetWB_MainMenu)))))

(fn NpcQuestStart
  (params (QuestName :type String) (Npc :type BP%20NPC%20Object%20Reference))
  (bind _wb_dialoguesystem (Variables|Default|GetWB_DialogueSystem))
  ;[1 1 1] 받은 Quest 이름 넘겨줌
  (Variables|/Game/Project/Widget/Popup/WB_DialogueSystem.WB_DialogueSystem_C|SetQuestName _wb_dialoguesystem QuestName)
  (Variables|/Game/Project/Widget/Popup/WB_DialogueSystem.WB_DialogueSystem_C|SetNpc _wb_dialoguesystem Npc))

(fn DialogueButtonUnbinding
  (Default|NpcDialogueButtonUnbinding (Variables|Default|GetWB_MainMenu)))