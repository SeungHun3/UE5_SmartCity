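; BP_HTTPRequest is an actor that handles HTTP callbacks carrying friends' last login times.
; Its SettingFriend event passes each UserID and time to the PlayFab component on the player's BP_LoginPawn.
; Each successful update decrements HttpCallCount, and the friend list refreshes only when that count reaches zero, batching the responses into one update.
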(event EventSettingFriend
  (params (UserID :type String) (LastLoginTime :type Date%20Time%20Structure%20%28by%20ref%29))
  ;[1 1 1] HTTP로 요청한 Friend의 로그아웃 정보를 콜백
  (bind _asbp_login_pawn (Utilities|Casting|CastToBP_LoginPawn (Pawn|GetControlledPawn (Game|GetPlayerController 0))))
  ;[1 1 1] 친구목록에 업데이트하기
  (bind _returnvalue (Class|ActorComponentPlayfab|UpdateFriendLoginTime (Variables|/Script/Test_LidarSample.Pawn_Player|GetBP_ActorComponent_Playfab _asbp_login_pawn) UserID LastLoginTime))
  (if _returnvalue
    (bind _result (Math|Integer|DecrementInt (Variables|Default|GetHttpCallCount))
      (:%20%20
        ;[1 1 1] HTTP로 요청이 모두 끝나면 그때 친구목록창을 갱신한다.
        (if (== _result 0)
          (Class|ActorComponentPlayfab|CallUpdateFriend (Variables|/Script/Test_LidarSample.Pawn_Player|GetBP_ActorComponent_Playfab _asbp_login_pawn)))))))

(fn ConstructionScript)